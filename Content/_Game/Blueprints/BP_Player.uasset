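; Player character Blueprint built from modular body meshes and a face with hair LOD handling.
; The construction script makes the torso, legs and feet meshes follow the main Mesh's pose through leader pose.
; On BeginPlay, HairLODSetup checks hair strand support; without it, it copies opacity values from the high-LOD eyelash dynamic material to the standard one, keeping fused eyelashes visible on lower LODs.
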(event EventBeginPlay
  (CallFunction|HairLODSetup))

(event Collision|EventActorBeginOverlap
  (params (OtherActor :type Actor%20Object%20Reference)))

(event EventTick
  (params (DeltaSeconds :type Float%20%28single-precision%29)))

(fn ConstructionScript
  (Components|SkinnedMesh|SetLeaderPoseComponent (Variables|Default|GetTorsoMesh) (Variables|Character|GetMesh) false false))

(fn HairLODSetup
  (bind _returnvalue (Class|GroomBlueprintLibrary|IsHairStrandsSupportedinWorld))
  (if (not _returnvalue) ; If strands are disabled then make fused eyelashes visible on lower LODs
    (bind _asmaterial_instance_dynamic (Utilities|Casting|CastToMaterialInstanceDynamic (Class|PrimitiveComponent|GetMaterialbyName (Variables|Default|GetFace) (Variables|Default|GetEyelashes%20HiLOD%20Material%20Slot))))
    (bind _asmaterial_instance_dynamic_2 (Utilities|Casting|CastToMaterialInstanceDynamic (Class|PrimitiveComponent|GetMaterialbyName (Variables|Default|GetFace) (Variables|Default|GetEyelashes%20Material%20%20Slot))))
    (bind _returnvalue_2 (Rendering|Material|GetScalarParameterValue _asmaterial_instance_dynamic "Opacity" :!class /Script/Engine.MaterialInstanceDynamic))
    (Rendering|Material|SetScalarParameterValue _asmaterial_instance_dynamic_2 "Opacity" _returnvalue_2 :!class /Script/Engine.MaterialInstanceDynamic)
    (bind _returnvalue_3 (Rendering|Material|GetScalarParameterValue _asmaterial_instance_dynamic "OpacityRT" :!class /Script/Engine.MaterialInstanceDynamic))
    (Rendering|Material|SetScalarParameterValue _asmaterial_instance_dynamic_2 "OpacityRT" _returnvalue_3 :!class /Script/Engine.MaterialInstanceDynamic)))